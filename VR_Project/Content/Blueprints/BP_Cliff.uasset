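; BP_Cliff is a level prop that lights a row of paired lamps in sequence when something overlaps its trigger box.
; The Box overlap event starts four left and right lamp pairs, one pair after another with short delays between them.
; StartLight casts each lamp's child actor to BP_Magic_04 and activates its particles.
; The overlap is not filtered by actor type.
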(event `self.ReceiveBeginPlay`)

(event `self.ReceiveActorBeginOverlap`
  (params (OtherActor :type "Actor Object Reference")))

(event `self.ReceiveTick`
  (params (DeltaSeconds :type "Float (single-precision)")))

(event `self.Box.OnComponentBeginOverlap`
  (params (OtherActor :type "Actor Object Reference") (OtherComp :type "PrimitiveComponent Object Reference") (OtherBodyIndex :type Integer) (bFromSweep :type Boolean) (SweepResult :type "EngineTypes.HitResult Structure (by ref)"))
  (`self.StartLight` (`self.L_Lamp1`))
  (`self.StartLight` (`self.R_Lamp1`))
  (`KismetSystemLibrary.Delay` 0.2)
  (`self.StartLight` (`self.L_Lamp2`))
  (`self.StartLight` (`self.R_Lamp2`))
  (`KismetSystemLibrary.Delay` 0.2)
  (`self.StartLight` (`self.L_Lamp3`))
  (`self.StartLight` (`self.R_Lamp3`))
  (`KismetSystemLibrary.Delay` 0.2)
  (`self.StartLight` (`self.L_Lamp4`))
  (`self.StartLight` (`self.R_Lamp4`)))

(fn `StartLight`
  (params (LightActor :type "ChildActorComponent Object Reference"))
  (bind _asbp_magic_04 (cast `/Game/CCCPRobot/BluePrint_Particles/BP_Magic_04` (`ChildActorComponent.ChildActor` LightActor))
    (:`then`
      (`/Game/CCCPRobot/BluePrint_Particles/BP_Magic_04.ActivateParticles` _asbp_magic_04))
    (:`CastFailed`
      _))
  (return))

(fn `UserConstructionScript`)