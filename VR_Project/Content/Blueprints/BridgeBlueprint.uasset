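; A gesture-driven bridge that the player raises by making a creation gesture within range.
; Creation hides the remote player's hint and plays the build animation once, then after a four-second delay re-enables the game mode's movement logic if the bridge is active.
; A one-shot DestroyBridge function plays the destruction animation and fires a magic particle child actor, but nothing in this graph calls it.
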(event `self.gestureEvent`
  (params (type :type "/Game/GestureEvent Enum" :default "NewEnumerator0"))
  (bind _inrange (`/Game/DistanceUtils.IsPlayerInRange` (`self.gestureRange`) self))
  (if _inrange
    (switch `/Game/GestureEvent` type
      (:`NewEnumerator0`
        (`self.Hide Creation Hint`)
        (`self.CreateBridge`)
        (`KismetSystemLibrary.Delay` 4.0)
        (bind _asmain_game_mode (cast `/Game/FirstPerson/Blueprints/mainGameMode` (`GameplayStatics.GetGameMode`)))
        (if (`self.isActive`)
          (set `/Game/Blueprints/Logic/MovementLogic.IsEnable` true (`/Game/FirstPerson/Blueprints/mainGameMode.MovementLogicRef` _asmain_game_mode))
          (set `self.isActive` false))))))

(fn `CreateBridge`
  (if (not (`self.isCreated`))
    (`SkeletalMeshComponent.PlayAnimation` (`self.SkeletalMeshComponent`) "/Game/Models/Bridge/Animation/BridgeCreation_Anim.BridgeCreation_Anim" false)
    (`SkeletalMeshComponent.SetPlayRate` self 1.25)
    (set `self.isCreated` true)))

(fn `DestroyBridge`
  (if (not (`self.isDestroyed`))
    (`SkeletalMeshComponent.PlayAnimation` (`self.SkeletalMeshComponent`) "/Game/Models/Bridge/Animation/BridgeDestruction_Anim.BridgeDestruction_Anim" false)
    (`SkeletalMeshComponent.SetPlayRate` self 1.25)
    (bind _asbp_magic_10 (cast `/Game/CCCPRobot/BluePrint_Particles/BP_Magic_10` (`ChildActorComponent.ChildActor` (`self.MagicBang`))))
    (`/Game/CCCPRobot/BluePrint_Particles/BP_Magic_10.ActivateParticle` _asbp_magic_10)
    (set `self.isDestroyed` true)))

(fn `Hide Creation Hint`
  (bind _asmain_game_mode (cast `/Game/FirstPerson/Blueprints/mainGameMode` (`GameplayStatics.GetGameMode`))
    (:`then`
      (bind _player (`/Game/FirstPerson/Blueprints/mainGameMode.getPlayer` _asmain_game_mode))
      (bind _asbp_remote_player (cast `/Game/Blueprints/BP_RemotePlayer` _player)
        (:`then`
          (`/Game/Blueprints/BP_RemotePlayer.HideCreationHint` _asbp_remote_player))
        (:`CastFailed`
          _)))
    (:`CastFailed`
      _))
  (return))

(fn `UserConstructionScript`)