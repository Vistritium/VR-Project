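; BP_RemotePlayer is an actor that shows gesture hints and the ending light in response to game progression facts.
; On BeginPlay it registers with mainGameMode as a progress listener, and FactWasAdded dispatches each fact name to a helper function.
; Each helper casts a child actor component to show or destroy the hands-up and hand-open indicators, or to finish the ending light.
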(event `self.ReceiveBeginPlay`
  (bind _asmain_game_mode (cast `/Game/FirstPerson/Blueprints/mainGameMode` (`GameplayStatics.GetGameMode`)))
  (`/Game/FirstPerson/Blueprints/mainGameMode.RegisterProgressListener` _asmain_game_mode self))

(event `self.FactWasAdded`
  (params (FactName :type "/Game/Blueprints/Logic/ProgressionSystem/E_Facts Enum" :default "NewEnumerator0"))
  (switch `/Game/Blueprints/Logic/ProgressionSystem/E_Facts` FactName
    (:`NewEnumerator7`
      (`self.StartEndingLight`))
    (:`NewEnumerator8`
      (`self.ShowCreationHint`))
    (:`NewEnumerator9`
      (`self.HideCreationHint`))
    (:`NewEnumerator10`
      (`self.ShowOpenHint`))
    (:`NewEnumerator11`
      (`self.HideOpenHint`))))

(fn `HideCreationHint`
  (bind _ashands_up_indicator (cast `/Game/handsUpIndicator` (`ChildActorComponent.ChildActor` (`self.CreationHand`))))
  (`/Game/handsUpIndicator.DestroyMe` _ashands_up_indicator))

(fn `HideOpenHint`
  (bind _ashand_open_indicator (cast `/Game/handOpenIndicator` (`ChildActorComponent.ChildActor` (`self.HandOpen`))))
  (`/Game/handOpenIndicator.DestroyMe` _ashand_open_indicator))

(fn `ShowCreationHint`
  (bind _ashands_up_indicator (cast `/Game/handsUpIndicator` (`ChildActorComponent.ChildActor` (`self.CreationHand`))))
  (`/Game/handsUpIndicator.ShowMe` _ashands_up_indicator))

(fn `ShowOpenHint`
  (bind _ashand_open_indicator (cast `/Game/handOpenIndicator` (`ChildActorComponent.ChildActor` (`self.HandOpen`))))
  (`/Game/handOpenIndicator.ShowMe` _ashand_open_indicator))

(fn `StartEndingLight`
  (bind _asending_light (cast `/Game/endingLight` (`ChildActorComponent.ChildActor` (`self.EndingLight`))))
  (`/Game/endingLight.Finish` _asending_light))

(fn `UserConstructionScript`)