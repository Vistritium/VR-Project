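; A bridge object that collapses and rebuilds through skeletal mesh animations, driven by story progression and a player gesture.
; It registers with the game mode as a progress listener; while active, progression facts trigger destruction, with a magic particle burst and creation hint, or reconstruction.
; An in-range creation gesture plays the rebuild, deactivates fact reactions, posts hint-hide and terrain-destruction facts, then enables movement logic after a short delay.
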(event `self.ReceiveBeginPlay`
  ;[1 1 1] Begin play
  (bind _asmain_game_mode (cast `/Game/FirstPerson/Blueprints/mainGameMode` (`GameplayStatics.GetGameMode`)))
  (`/Game/FirstPerson/Blueprints/mainGameMode.RegisterProgressListener` _asmain_game_mode self))

(event `self.gestureEvent`
  (params (type :type "/Game/GestureEvent Enum" :default "NewEnumerator0"))
  (switch `/Game/GestureEvent` type
    (:`NewEnumerator0`
      (bind _inrange (`/Game/DistanceUtils.IsPlayerInRange` (`self.gestureRange`) self))
      (if _inrange
        (`self.CreateBridge`)
        (set `self.isActive` false)
        (bind _asmain_game_mode (cast `/Game/FirstPerson/Blueprints/mainGameMode` (`GameplayStatics.GetGameMode`)))
        (bind _progressionsystem (`/Game/FirstPerson/Blueprints/mainGameMode.ProgressionSystem` _asmain_game_mode))
        (`/Game/Blueprints/Logic/ProgressionSystem/BPI_ProgressionSystem.AddFact` _progressionsystem "NewEnumerator9")
        (`/Game/Blueprints/Logic/ProgressionSystem/BPI_ProgressionSystem.AddFact` _progressionsystem "NewEnumerator5")
        (`KismetSystemLibrary.Delay` 2.0)
        (set `/Game/Blueprints/Logic/MovementSystem/BP_MovementSystem.IsEnable` true (`/Game/FirstPerson/Blueprints/mainGameMode.MovementLogicRef` _asmain_game_mode))))))

(event `self.FactWasAdded`
  (params (FactName :type "/Game/Blueprints/Logic/ProgressionSystem/E_Facts Enum" :default "NewEnumerator0"))
  (if (`self.isActive`)
    (switch `/Game/Blueprints/Logic/ProgressionSystem/E_Facts` FactName
      (:`NewEnumerator0`
        (`self.DestroyBridge`)
        (bind _asmain_game_mode (cast `/Game/FirstPerson/Blueprints/mainGameMode` (`GameplayStatics.GetGameMode`)))
        (`/Game/Blueprints/Logic/ProgressionSystem/BPI_ProgressionSystem.AddFact` (`/Game/FirstPerson/Blueprints/mainGameMode.ProgressionSystem` _asmain_game_mode) "NewEnumerator8"))
      (:`NewEnumerator1`
        (`self.CreateBridge`)))))

(fn `CreateBridge`
  (if (not (`self.isCreated`))
    (`SkeletalMeshComponent.PlayAnimation` (`self.SkeletalMeshComponent`) "/Game/Models/LongerBridge/Animation/LongerBridgeCreation_Anim.LongerBridgeCreation_Anim" false)
    (set `self.isCreated` true)))

(fn `DestroyBridge`
  (if (not (`self.isDestroyed`))
    (`SkeletalMeshComponent.PlayAnimation` (`self.SkeletalMeshComponent`) "/Game/Models/LongerBridge/Animation/LongerBridgeDestruction_Anim.LongerBridgeDestruction_Anim" false)
    (bind _asbp_magic_10 (cast `/Game/Particles/BluePrint_Particles/BP_Magic_10` (`ChildActorComponent.ChildActor` (`self.MagicBang`))))
    (`/Game/Particles/BluePrint_Particles/BP_Magic_10.ActivateParticle` _asbp_magic_10)
    (set `self.isDestroyed` true)))

(fn `UserConstructionScript`)