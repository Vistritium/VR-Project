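; Start cylinder actor that spins, registers itself with mainGameMode, and hands off to the game mode's StartCamera after a timed spin-up.
; It rotates every tick around its initial forward axis, accelerating exponentially up to a cap once Start is called.
; Delays trigger the camera call and, shortly before it, a light transition driven through the TheLight material parameter collection.
; As a progress listener, it destroys itself when a specific fact is added.
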(event `self.ReceiveBeginPlay`
  ;[1 1 1] Begin play
  (set `self.forward` (`KismetMathLibrary.GetForwardVector` (`self.K2_GetActorRotation`)))
  (set `self.beginRotationFactor` (`self.rotationFactor`))
  (bind _asmain_game_mode (cast `/Game/FirstPerson/Blueprints/mainGameMode` (`GameplayStatics.GetGameMode`)))
  (set `/Game/FirstPerson/Blueprints/mainGameMode.startCylinder` self _asmain_game_mode)
  (`/Game/FirstPerson/Blueprints/mainGameMode.RegisterProgressListener` _asmain_game_mode self))

(event `self.ReceiveTick`
  (params (DeltaSeconds :type "Float (single-precision)"))
  (bind _lightcurrenttransition (`self.lightCurrentTransition`))
  (bind _rotationcap (`self.rotationCap`))
  ;[1 1 1] Tick
  (set `self.deltaSeconds` DeltaSeconds)
  (`|ExecutionSequence`
    (:`then_0`
      (if (`self.started`)
        (`|ExecutionSequence`
          (:`then_0`
            (bind _output_get (set `self.rotationFactor` (+ (`self.rotationFactor`) (* (`self.deltaSeconds`) (* (`self.rotationFactor`) (`self.increaseValue`))))))
            (`/Engine/EditorBlueprintResources/StandardMacros.CompareFloat` _output_get _rotationcap
              (:`>`
                (set `self.rotationFactor` _rotationcap))))
          (:`then_1`
            (`/Engine/EditorBlueprintResources/StandardMacros.DoOnce` false
              (:`Completed`
                (`|ExecutionSequence`
                  (:`then_0`
                    (`KismetSystemLibrary.Delay` (`self.duration`))
                    (`self.Stop`))
                  (:`then_1`
                    (`KismetSystemLibrary.Delay` (- (`self.duration`) (`self.lightValueTransitionDuration`)))
                    (`self.StartLightTransition`))))))
          (:`then_2`
            (if (`self.lightTransitionStarted`)
              (`|ExecutionSequence`
                (:`then_0`
                  (set `self.lightCurrentTransition` (+ (`self.deltaSeconds`) (`self.lightCurrentTransition`))))
                (:`then_1`
                  (`KismetMaterialLibrary.SetScalarParameterValue` "/Game/Blueprints/TheLight.TheLight" "Light" (`KismetMathLibrary.Lerp` (`self.startLightValue`) (`self.finishLightValue`) _lightcurrenttransition))
                  (`KismetMaterialLibrary.SetScalarParameterValue` "/Game/Blueprints/TheLight.TheLight" "interpolationFactor" _lightcurrenttransition))))))))
    (:`then_1`
      (`SceneComponent.K2_AddLocalRotation` (`KismetMathLibrary.RotatorFromAxisAndAngle` (`self.forward`) (* (`self.deltaSeconds`) (`self.rotationFactor`)))))))

(event `self.FactWasAdded`
  (params (FactName :type "/Game/Blueprints/Logic/ProgressionSystem/E_Facts Enum" :default "NewEnumerator0"))
  (if (`|EnumEquality` FactName "NewEnumerator3")
    (`self.K2_DestroyActor`)))

(fn `CheckFactExists`
  (params (FactName :type "/Game/Blueprints/Logic/ProgressionSystem/E_Facts Enum" :default "NewEnumerator0"))
  (returns (FactExists :type Boolean))
  (return false))

(fn `Start`
  (set `self.started` true))

(fn `StartLightTransition`
  (set `self.lightTransitionStarted` true))

(fn `Stop`
  (bind _asmain_game_mode (cast `/Game/FirstPerson/Blueprints/mainGameMode` (`GameplayStatics.GetGameMode`)))
  (`/Game/FirstPerson/Blueprints/mainGameMode.startCamera` _asmain_game_mode))

(fn `UserConstructionScript`)