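; Sun object that unfurls and spins on a creation gesture, then folds up after a destruction gesture.
; A delay loop replays the spin animation and checks the Destroyed flag each cycle, folding by playing the unfurl animation in reverse.
; It registers as a progress listener with the game mode, and the "Sun Burn" fact activates particles on its BP_Magic_09 child actor.
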(event `self.ReceiveBeginPlay`
  (bind _asmain_game_mode (cast `/Game/FirstPerson/Blueprints/mainGameMode` (`GameplayStatics.GetGameMode`)))
  (`/Game/FirstPerson/Blueprints/mainGameMode.RegisterProgressListener` _asmain_game_mode self))

(event `self.gestureEvent`
  (params (type :type "/Game/GestureEvent Enum" :default "NewEnumerator0"))
  (bind _destroyed (`self.destroyed`))
  (bind _skeletalmeshcomponent (`self.SkeletalMeshComponent`))
  (bind _skeletalmeshcomponent_2 (`self.SkeletalMeshComponent`))
  (switch `/Game/GestureEvent` type
    (:`NewEnumerator0`
      (if _destroyed
        (set `self.destroyed` false)
        (`SkeletalMeshComponent.PlayAnimation` _skeletalmeshcomponent_2 "/Game/Models/Background/Sun/Animations/Animation_Unfurl_Anim.Animation_Unfurl_Anim" false)
        (`SkeletalMeshComponent.SetPlayRate` _skeletalmeshcomponent_2 1.0)
        (`KismetSystemLibrary.Delay` 2.0)
        (`SkeletalMeshComponent.PlayAnimation` _skeletalmeshcomponent_2 "/Game/Models/Background/Sun/Animations/Animation_Spin_Anim.Animation_Spin_Anim" false)
        (`KismetSystemLibrary.Delay` 1.667 :!label _label)
        (if (`self.destroyed`)
          (`SkeletalMeshComponent.PlayAnimation` _skeletalmeshcomponent "/Game/Models/Background/Sun/Animations/Animation_Unfurl_Anim.Animation_Unfurl_Anim" false)
          (`SkeletalMeshComponent.SetPosition` _skeletalmeshcomponent 100.0 true)
          (`SkeletalMeshComponent.SetPlayRate` _skeletalmeshcomponent -0.3)
          (else
            (`SkeletalMeshComponent.PlayAnimation` _skeletalmeshcomponent "/Game/Models/Background/Sun/Animations/Animation_Spin_Anim.Animation_Spin_Anim" false)
            (goto _label)))))
    (:`NewEnumerator1`
      (if (not _destroyed)
        (set `self.destroyed` true)))))

(event `self.FactWasAdded`
  (params (FactName :type "/Game/Blueprints/Logic/ProgressionSystem/E_Facts Enum" :default "NewEnumerator0"))
  (switch `/Game/Blueprints/Logic/ProgressionSystem/E_Facts` FactName
    (:`NewEnumerator15`
      (`self.BurnTheSun`))))

(fn `BurnTheSun`
  (bind _asbp_magic_09 (cast `/Game/Particles/BluePrint_Particles/BP_Magic_09` (`ChildActorComponent.ChildActor` (`self.MagicParticles`))))
  (`/Game/Particles/BluePrint_Particles/BP_Magic_09.ActivateParticles` _asbp_magic_09))

(fn `UserConstructionScript`)