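; Pyramid object with a skeletal mesh that unfurls and folds up in response to creation and destruction gestures.
; Creation plays the unfurl animation, then a looping bounce that freezes after a short delay unless destroyed meanwhile.
; Destruction plays the unfurl in reverse, with a Destroyed flag blocking repeats of either gesture.
; Separately, SequenceStart waits TimeToDestroy before calling ScaleDestroy.
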(event `self.SequenceStart`
  (`KismetSystemLibrary.Delay` (`self.timeToDestroy`))
  (`/Game/scaleDestroyer.scaleDestroy` 4.0))

(event `self.gestureEvent`
  (params (type :type "/Game/GestureEvent Enum" :default "NewEnumerator0"))
  (bind _skeletalmeshcomponent (`self.SkeletalMeshComponent`))
  (bind _skeletalmeshcomponent_2 (`self.SkeletalMeshComponent`))
  (switch `/Game/GestureEvent` type
    (:`NewEnumerator0`
      (if (`self.destroyed`)
        (set `self.destroyed` false)
        (`SkeletalMeshComponent.PlayAnimation` _skeletalmeshcomponent_2 "/Game/Models/Background/Pyramid/Animations/Anim_Unfurl_Anim.Anim_Unfurl_Anim" false)
        (`SkeletalMeshComponent.SetPlayRate` _skeletalmeshcomponent_2 1.0)
        (`KismetSystemLibrary.Delay` 1.0)
        (`SkeletalMeshComponent.PlayAnimation` _skeletalmeshcomponent_2 "/Game/Models/Background/Pyramid/Animations/Anim_Bounce_Anim.Anim_Bounce_Anim" true)
        (`KismetSystemLibrary.Delay` 2.0)
        (if (not (`self.destroyed`))
          (`SkeletalMeshComponent.SetPlayRate` (`self.SkeletalMeshComponent`) 0.0))))
    (:`NewEnumerator1`
      (if (not (`self.destroyed`))
        (set `self.destroyed` true)
        (`SkeletalMeshComponent.PlayAnimation` _skeletalmeshcomponent "/Game/Models/Background/Pyramid/Animations/Anim_Unfurl_Anim.Anim_Unfurl_Anim" false)
        (`SkeletalMeshComponent.SetPosition` _skeletalmeshcomponent 100.0 true)
        (`SkeletalMeshComponent.SetPlayRate` _skeletalmeshcomponent -1.0)))))

(fn `UserConstructionScript`)