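; Star actor that orbits a point around the Z axis while spinning on its own local axis, reacting to music beats and gestures.
; It registers with mainGameMode as a beat receiver and picks a new random spin axis on each big beat.
; Creation and destruction gestures toggle its Destroyed state, playing Star_Anim forward to create it and in reverse to destroy it.
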(event `self.ReceiveBeginPlay`
  (bind _asmain_game_mode (cast `/Game/FirstPerson/Blueprints/mainGameMode` (`GameplayStatics.GetGameMode`)))
  (`/Game/FirstPerson/Blueprints/mainGameMode.addNewBeatReceiver` _asmain_game_mode self))

(event `self.ReceiveActorBeginOverlap`
  (params (OtherActor :type "Actor Object Reference")))

(event `self.ReceiveTick`
  (params (DeltaSeconds :type "Float (single-precision)"))
  (bind _aroundpoint (`self.aroundPoint`))
  (`|ExecutionSequence`
    (:`then_0`
      (`self.K2_SetActorLocation` (+ (`KismetMathLibrary.RotateAngleAxis` (- (`self.K2_GetActorLocation` self) _aroundpoint) (* DeltaSeconds 10.0) (0.0 0.0 1.0)) _aroundpoint)))
    (:`then_1`
      (`SceneComponent.K2_AddLocalRotation` (`KismetMathLibrary.RotatorFromAxisAndAngle` (`self.rotateVector`) (* (`self.rotateSelfFactor`) DeltaSeconds))))))

(event `self.gestureEvent`
  (params (type :type "/Game/GestureEvent Enum" :default "NewEnumerator0"))
  (switch `/Game/GestureEvent` type
    (:`NewEnumerator0`
      (if (`self.destroyed`)
        (set `self.destroyed` false)
        (`SkeletalMeshComponent.PlayAnimation` self "/Game/Models/Background/Star/Animations/Star_Anim.Star_Anim" false)
        (`SkeletalMeshComponent.SetPlayRate` self 1.0)))
    (:`NewEnumerator1`
      (if (not (`self.destroyed`))
        (set `self.destroyed` true)
        (`SkeletalMeshComponent.PlayAnimation` self "/Game/Models/Background/Star/Animations/Star_Anim.Star_Anim" false)
        (`SkeletalMeshComponent.SetPosition` (`self.SkeletalMeshComponent`) 100.0 true)
        (`SkeletalMeshComponent.SetPlayRate` self -1.0)))))

(event `self.beat`
  (params (beat :type "/Game/FirstPerson/Blueprints/BEAT Enum" :default "NewEnumerator0") (factor :type "Float (single-precision)"))
  (switch `/Game/FirstPerson/Blueprints/BEAT` beat
    (:`NewEnumerator1`
      (set `self.rotateVector` (`KismetMathLibrary.RandomUnitVector`)))))

(fn `UserConstructionScript`)