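; Tree Blueprint that grows and un-grows through animation in response to creation and destruction gesture events.
; A Destroyed flag gates each gesture: creation plays the spin-growth animation forward, destruction runs it backward with a negative play rate.
; Separate one-shot functions offer spin or normal growth, guarded by IsReady.
; After a short delay from BeginPlay, it stops BeatScalePulser and triggers ScaleDestroyer's timed scale-destroy.
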(event `self.ReceiveBeginPlay`
  (`KismetSystemLibrary.Delay` 4.0)
  (`/Game/beatScalePulser.stop` (`self.beatScalePulser`))
  (`/Game/scaleDestroyer.scaleDestroy` (`self.scaleDestroyer`) 5.0))

(event `self.gestureEvent`
  (params (type :type "/Game/GestureEvent Enum" :default "NewEnumerator0"))
  (bind _tree (`self.Tree`))
  (bind _destroyed (`self.destroyed`))
  (switch `/Game/GestureEvent` type
    (:`NewEnumerator0`
      (if _destroyed
        (set `self.destroyed` false)
        (if (`KismetMathLibrary.RandomBool`)
          (`SkeletalMeshComponent.PlayAnimation` _tree "/Game/Models/Tree/Animation/TreeSpinGrowth_Anim.TreeSpinGrowth_Anim" false)
          (else
            (`SkeletalMeshComponent.PlayAnimation` _tree "/Game/Models/Tree/Animation/TreeSpinGrowth_Anim.TreeSpinGrowth_Anim" false)))
        (`SkeletalMeshComponent.SetPlayRate` _tree 1.0)))
    (:`NewEnumerator1`
      (if (not _destroyed)
        (set `self.destroyed` true)
        (if false
          (`SkeletalMeshComponent.PlayAnimation` _tree "/Game/Models/Tree/Animation/TreeSpinGrowth_Anim.TreeSpinGrowth_Anim" false)
          (else
            (`SkeletalMeshComponent.PlayAnimation` _tree "/Game/Models/Tree/Animation/TreeSpinGrowth_Anim.TreeSpinGrowth_Anim" false)))
        (`SkeletalMeshComponent.SetPosition` 100.0)
        (`SkeletalMeshComponent.SetPlayRate` _tree -1.0)))))

(fn `SimpleGrowTree`
  (if (not (`self.IsReady`))
    (`SkeletalMeshComponent.PlayAnimation` (`self.Tree`) "/Game/Models/Tree/Animation/TreeNormalGrowth_Anim.TreeNormalGrowth_Anim" false)
    (set `self.IsReady` true)))

(fn `SpinGrowTree`
  (if (not (`self.IsReady`))
    (`SkeletalMeshComponent.PlayAnimation` (`self.Tree`) "/Game/Models/Tree/Animation/TreeSpinGrowth_Anim.TreeSpinGrowth_Anim" false)
    (set `self.IsReady` true)))

(fn `UserConstructionScript`)