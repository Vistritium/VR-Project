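; Final gate actor that opens when the player performs an OPEN gesture within its gesture range.
; The gesture plays the gate's skeletal animation once, guarded by an IsOpened flag, then turns off the previous pair of lamps and activates particles on the left and right magic lamps, all via child actors.
; After a short delay it enables the main game mode's movement logic.
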(event `self.gestureEvent`
  (params (type :type "/Game/GestureEvent Enum" :default "NewEnumerator0"))
  (bind _inrange (`/Game/DistanceUtils.IsPlayerInRange` (`self.GestureRange`) self))
  (if _inrange
    (switch `/Game/GestureEvent` type
      (:`NewEnumerator2`
        (`self.OpenGate`)
        (`self.DeactivatePreviousLamps`)
        (`self.ActivateMagicLamps`)
        (`KismetSystemLibrary.Delay` 2.5)
        (bind _asmain_game_mode (cast `/Game/FirstPerson/Blueprints/mainGameMode` (`GameplayStatics.GetGameMode`)))
        (set `/Game/Blueprints/Logic/MovementLogic.IsEnable` true (`/Game/FirstPerson/Blueprints/mainGameMode.MovementLogicRef` _asmain_game_mode))))))

(fn `ActivateMagicLamps`
  (bind _asbp_magic_05 (cast `/Game/CCCPRobot/BluePrint_Particles/BP_Magic_05` (`ChildActorComponent.ChildActor` (`self.LeftMagicLamp`))))
  (`/Game/CCCPRobot/BluePrint_Particles/BP_Magic_05.ActivateParticles` _asbp_magic_05)
  (bind _asbp_magic_05_2 (cast `/Game/CCCPRobot/BluePrint_Particles/BP_Magic_05` (`ChildActorComponent.ChildActor` (`self.RightMagicLamp`))))
  (`/Game/CCCPRobot/BluePrint_Particles/BP_Magic_05.ActivateParticles` _asbp_magic_05_2))

(fn `DeactivatePreviousLamps`
  (bind _asbp_magic_03 (cast `/Game/CCCPRobot/BluePrint_Particles/BP_Magic_03` (`ChildActorComponent.ChildActor` (`self.PreviousLeftLamp`))))
  (`ActorComponent.Deactivate` _asbp_magic_03)
  (bind _asbp_magic_03_2 (cast `/Game/CCCPRobot/BluePrint_Particles/BP_Magic_03` (`ChildActorComponent.ChildActor` (`self.PreviousRightLamp`))))
  (`ActorComponent.Deactivate` _asbp_magic_03_2))

(fn `OpenGate`
  (if (not (`self.IsOpened`))
    (`SkeletalMeshComponent.PlayAnimation` (`self.SkeletalMeshComponent`) "/Game/Models/Gate/Animation/GateFinal_Anim.GateFinal_Anim" false)
    (set `self.IsOpened` true)))

(fn `UserConstructionScript`)