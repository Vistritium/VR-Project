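; BP_ProgressionSystem tracks game progression as a list of named facts.
; AddFact appends a fact only if it is not already present, then fires FactWasAdded with its name to announce the change.
; CheckFactExists reports whether a given fact is in the list, and the file contains no logic for removing facts.
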(event `self.AddFact`
  (params (FactName :type "/Game/Blueprints/Logic/ProgressionSystem/E_Facts Enum" :default "NewEnumerator0"))
  (if (== (`KismetArrayLibrary.Array_Find` (`self.Facts`) FactName) -1)
    (`KismetArrayLibrary.Array_Add` (`self.Facts`) FactName)
    (`self.FactWasAdded` FactName)))

(fn `CheckFactExists`
  (params (FactName :type "/Game/Blueprints/Logic/ProgressionSystem/E_Facts Enum" :default "NewEnumerator0"))
  (returns (FactExists :type Boolean))
  (return (!= (`KismetArrayLibrary.Array_Find` (`self.Facts`) FactName) -1)))

(fn `UserConstructionScript`)