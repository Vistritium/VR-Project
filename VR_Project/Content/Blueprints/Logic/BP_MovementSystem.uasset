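; VR on-rails movement system that carries the game mode's active camera along indexed BP_MovementTargetPoint actors while its rotation follows the headset.
; BeginPlay gathers the points, snaps the camera to the first and hides player hints.
; Tick steps the camera by Speed per frame, without delta time, advancing the target within 50 units.
; Point flags halt movement or teleport the camera, and running out of points triggers BP_RemotePlayer's ending light.
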(event EventBeginPlay
  (CallFunction|ResetHeadDeviceTransform)
  (CallFunction|GatherAllMovementPointsfromScene)
  (CallFunction|InitializeVariables)
  (CallFunction|SetInitialPosition)
  (CallFunction|UpdateBorderPoints)
  (CallFunction|CheckStopMovementCondition)
  (CallFunction|UpdateMovementPosition)
  (CallFunction|HideHints))

(event EventTick
  (params (DeltaSeconds :type Float%20%28single-precision%29))
  (CallFunction|UpdateTransformationfromHeadDevice)
  (if (Variables|Default|GetIsEnable)
    (if (< (Math|Vector|VectorLength (- (Variables|Default|GetNextPosition) (Transformation|GetActorLocation (Variables|Default|GetActiveCamera)))) 5e+01)
      (CallFunction|CheckStopMovementCondition)
      (CallFunction|SetNewNextMovementPoint)
      (CallFunction|CheckImediatteMovementCondition)
      (CallFunction|CheckLastPointCondition)
      (CallFunction|UpdateBorderPoints)
      (else
        (CallFunction|UpdateMovementPosition)))))

(fn ConstructionScript)

(fn GatherAllMovementPointsfromScene
  (bind _outactors (Actor|GetAllActorsOfClass "/Game/Blueprints/BP_MovementTargetPoint.BP_MovementTargetPoint_C"))
  (Variables|Default|SetPoints _outactors))

(fn UpdateBorderPoints
  (bind _foundedactor (CallFunction|GetActorwithIndex (Variables|Default|GetCurrentIndex)))
  (Variables|Default|SetCurrentPosition (Transformation|GetActorLocation _foundedactor))
  (bind _foundedactor_2 (CallFunction|GetActorwithIndex (Variables|Default|GetNextIndex)))
  (Variables|Default|SetNextPosition (Transformation|GetActorLocation _foundedactor_2))
  (Variables|Default|SetMovementDirection (Math|Vector|Normalize (- (Variables|Default|GetNextPosition) (Variables|Default|GetCurrentPosition)))))

(fn GetActorwithIndex
  (params (Index :type Integer :default 0))
  (bind _points (Variables|Default|GetPoints))
  (bind _array_element (Utilities|Array|ForEachLoopwithBreak (Variables|Default|GetPoints) :!label _label)
    (:LoopBody
      (if (== (Variables|/Game/Blueprints/BP_MovementTargetPoint.BP_MovementTargetPoint_C|GetIndex _array_element) Index)
        (LocalVariables|SetInternalFoundedActor _array_element)
        (goto _label Break)))
    (:Completed
      (if (!= (LocalVariables|GetInternalFoundedActor) 0)
        _
        (else
          (LocalVariables|SetInternalFoundedActor (Utilities|Array|Get(acopy) _points (- (Utilities|Array|Length _points) 1)))))
      (return (LocalVariables|GetInternalFoundedActor)))))

(fn CheckStopMovementCondition
  (bind _foundedactor (CallFunction|GetActorwithIndex (Variables|Default|GetNextIndex)))
  (if (Variables|/Game/Blueprints/BP_MovementTargetPoint.BP_MovementTargetPoint_C|GetStopMovement _foundedactor)
    (Variables|Default|SetIsEnable false))
  (return))

(fn SetNewNextMovementPoint
  (Variables|Default|SetCurrentIndex (Variables|Default|GetNextIndex))
  (Variables|Default|SetNextIndex (+ 1 (Variables|Default|GetNextIndex)))
  (return))

(fn CheckLastPointCondition
  (if (>= (Variables|Default|GetNextIndex) (Utilities|Array|Length (Variables|Default|GetPoints)))
    (Variables|Default|SetNextIndex (Variables|Default|GetCurrentIndex))
    (bind _asmain_game_mode (Utilities|Casting|CastTomainGameMode (Game|GetGameMode))
      (:then
        (bind _player (Default|GetPlayer _asmain_game_mode))
        (bind _asbp_remote_player (Utilities|Casting|CastToBP_RemotePlayer _player)
          (:then
            (Default|StartEndingLight _asbp_remote_player))
          (:CastFailed
            _)))
      (:CastFailed
        _)))
  (return))

(fn SetInitialPosition
  (bind _foundedactor (CallFunction|GetActorwithIndex (Variables|Default|GetCurrentIndex)))
  (Transformation|SetActorTransform (Variables|Default|GetActiveCamera) (Transformation|GetActorTransform _foundedactor))
  (return))

(fn InitializeVariables
  (Variables|Default|SetCurrentIndex 0)
  (Variables|Default|SetNextIndex (+ (Variables|Default|GetCurrentIndex) 1))
  (bind _asmain_game_mode (Utilities|Casting|CastTomainGameMode (Game|GetGameMode))
    (:then
      (Variables|Default|SetActiveCamera (Variables|/Game/FirstPerson/Blueprints/mainGameMode.mainGameMode_C|GetActiveCamera _asmain_game_mode)))
    (:CastFailed
      _))
  (return))

(fn UpdateMovementPosition
  (Transformation|SetActorTransform (Variables|Default|GetActiveCamera) (Math|Transform|MakeTransform (+ (* (Variables|Default|GetMovementDirection) (Variables|Default|GetSpeed)) (Transformation|GetActorLocation (Variables|Default|GetActiveCamera))) (.DeviceRotation (Class|HeadMountedDisplayFunctionLibrary|GetOrientationandPosition)) "0, 0, 0"))
  (return))

(fn CheckImediatteMovementCondition
  (bind _foundedactor (CallFunction|GetActorwithIndex (Variables|Default|GetNextIndex)))
  (if (Variables|/Game/Blueprints/BP_MovementTargetPoint.BP_MovementTargetPoint_C|GetImmediateMovement _foundedactor)
    (CallFunction|UpdateBorderPoints)
    (Transformation|SetActorTransform (Variables|Default|GetActiveCamera) (Math|Transform|MakeTransform (Variables|Default|GetNextPosition) (.DeviceRotation (Class|HeadMountedDisplayFunctionLibrary|GetOrientationandPosition)) "0, 0, 0"))
    (CallFunction|SetNewNextMovementPoint))
  (return))

(fn UpdateTransformationfromHeadDevice
  (bind _activecamera (Variables|Default|GetActiveCamera))
  (Transformation|SetActorTransform _activecamera (Math|Transform|MakeTransform (Transformation|GetActorLocation _activecamera) (.DeviceRotation (Class|HeadMountedDisplayFunctionLibrary|GetOrientationandPosition))))
  (return))

(fn HideHints
  (bind _asmain_game_mode (Utilities|Casting|CastTomainGameMode (Game|GetGameMode))
    (:then
      (bind _player (Default|GetPlayer _asmain_game_mode))
      (bind _asbp_remote_player (Utilities|Casting|CastToBP_RemotePlayer _player)
        (:then
          (Default|HideCreationHint _asbp_remote_player)
          (Default|HideOpenHint _asbp_remote_player))
        (:CastFailed
          _)))
    (:CastFailed
      _))
  (return))

(fn ResetHeadDeviceTransform
  (Class|HeadMountedDisplayFunctionLibrary|ResetOrientationandPosition 0.0 "OrientationAndPosition")
  (return))