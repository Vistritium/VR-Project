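; MovementLogic moves the game mode's active camera between movement target points placed in the level.
; On BeginPlay it gathers all BP_MovementTargetPoint actors, snaps the camera to the first and caches the first two locations.
; While enabled, Tick lerps between them by elapsed time over MovementTime, converting only location to a transform.
; The timer runs even when disabled, and the indices never advance past that first segment.
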(event `self.ReceiveBeginPlay`
  (`self.GatherAllMovementPoints`)
  (set `self.CurrentIndex` 0)
  (set `self.NextIndex` (+ (`self.CurrentIndex`) 1))
  (bind _asmain_game_mode (cast `/Game/FirstPerson/Blueprints/mainGameMode` (`GameplayStatics.GetGameMode`)))
  (set `self.ActiveCamera` (`/Game/FirstPerson/Blueprints/mainGameMode.ActiveCamera` _asmain_game_mode))
  ;[1 1 1] Set initial position
  (`self.K2_SetActorTransform` (`self.ActiveCamera`) (`self.GetTransform` (`KismetArrayLibrary.Array_Get` (`self.Points`) (`self.CurrentIndex`))) false)
  (`self.UpdateBorderPoints`))

(event `self.ReceiveTick`
  (params (DeltaSeconds :type "Float (single-precision)"))
  (set `self.CurrentTime` (+ DeltaSeconds (`self.CurrentTime`)))
  (if (`self.IsEnable`)
    (`self.K2_SetActorTransform` (`self.ActiveCamera`) (`KismetMathLibrary.Conv_VectorToTransform` (`KismetMathLibrary.VLerp` (`self.CurrentPosition`) (`self.NextPosition`) (/ (`self.CurrentTime`) (`self.MovementTime`)))) false)))

(fn `GatherAllMovementPoints`
  (bind _outactors (`GameplayStatics.GetAllActorsOfClass` "/Game/Blueprints/BP_MovementTargetPoint.BP_MovementTargetPoint_C"))
  (set `self.Points` _outactors))

(fn `UpdateBorderPoints`
  (set `self.CurrentPosition` (`self.K2_GetActorLocation` (`KismetArrayLibrary.Array_Get` (`self.Points`) (`self.CurrentIndex`))))
  (set `self.NextPosition` (`self.K2_GetActorLocation` (`KismetArrayLibrary.Array_Get` (`self.Points`) (`self.NextIndex`)))))

(fn `UserConstructionScript`)