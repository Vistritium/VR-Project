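; VR on-rails movement system that carries the game mode's active camera along indexed BP_MovementTargetPoint actors while the headset drives rotation.
; Tick moves the camera toward the next point, interpolating speed by distance, without delta-time scaling.
; ChangeTargetPointToNext, not called here, advances the path, applying each point's stop, immediate-jump and progression-fact settings.
; Each point receives a reference to this system; Tick's proximity-based advance is disconnected.
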(event EventBeginPlay
  (CallFunction|ResetHeadDeviceTransform)
  (CallFunction|GatherAllMovementPointsfromScene)
  (CallFunction|InitializeVariables)
  (CallFunction|SetInitialPosition)
  (CallFunction|SetInitialSpeed)
  (CallFunction|UpdateBorderPoints)
  (CallFunction|CheckStopMovementCondition)
  (CallFunction|UpdateMovementPosition)
  (CallFunction|AddFactsfromCurrentPoint))

(event EventTick
  (params (DeltaSeconds :type Float%20%28single-precision%29))
  (CallFunction|UpdateTransformationfromHeadDevice)
  (if (Variables|Default|GetIsEnable)
    (CallFunction|UpdateMovementPosition)
    (CallFunction|UpdateMovementSpeed)))

(fn ConstructionScript)

(fn GatherAllMovementPointsfromScene
  (bind _outactors (Actor|GetAllActorsOfClass "/Game/Blueprints/Logic/MovementSystem/BP_MovementTargetPoint.BP_MovementTargetPoint_C"))
  (bind _output_get (Variables|Default|SetPoints _outactors))
  (for _array_element _output_get
    (Default|SetMovementSystem _array_element self)))

(fn UpdateBorderPoints
  (bind _foundedactor (CallFunction|GetActorwithIndex (Variables|Default|GetCurrentIndex)))
  (Variables|Default|SetCurrentPosition (Transformation|GetActorLocation _foundedactor))
  (bind _foundedactor_2 (CallFunction|GetActorwithIndex (Variables|Default|GetNextIndex)))
  (Variables|Default|SetNextPosition (Transformation|GetActorLocation _foundedactor_2))
  (Variables|Default|SetMovementDirection (Math|Vector|Normalize (- (Variables|Default|GetNextPosition) (Variables|Default|GetCurrentPosition)))))

(fn GetActorwithIndex
  (params (Index :type Integer :default 0))
  (bind _points (Variables|Default|GetPoints))
  (bind _array_element (Utilities|Array|ForEachLoopwithBreak (Variables|Default|GetPoints) :!label _label)
    (:LoopBody
      (if (== (Variables|/Game/Blueprints/Logic/MovementSystem/BP_MovementTargetPoint.BP_MovementTargetPoint_C|GetIndex _array_element) Index)
        (LocalVariables|SetInternalFoundedActor _array_element)
        (goto _label Break)))
    (:Completed
      (if (!= (LocalVariables|GetInternalFoundedActor) 0)
        _
        (else
          (LocalVariables|SetInternalFoundedActor (Utilities|Array|Get(acopy) _points (- (Utilities|Array|Length _points) 1)))))
      (return (LocalVariables|GetInternalFoundedActor)))))

(fn CheckStopMovementCondition
  (bind _foundedactor (CallFunction|GetActorwithIndex (Variables|Default|GetNextIndex)))
  (if (Variables|/Game/Blueprints/Logic/MovementSystem/BP_MovementTargetPoint.BP_MovementTargetPoint_C|GetStopMovement _foundedactor)
    (Variables|Default|SetIsEnable false))
  (return))

(fn SetNewNextMovementPoint
  (Variables|Default|SetCurrentIndex (Variables|Default|GetNextIndex))
  (Variables|Default|SetNextIndex (+ 1 (Variables|Default|GetNextIndex)))
  (return))

(fn CheckLastPointCondition
  (if (>= (Variables|Default|GetNextIndex) (Utilities|Array|Length (Variables|Default|GetPoints)))
    (Variables|Default|SetNextIndex (Variables|Default|GetCurrentIndex))
    (bind _asmain_game_mode (Utilities|Casting|CastTomainGameMode (Game|GetGameMode))
      (:then
        (Default|AddFact (Variables|/Game/FirstPerson/Blueprints/mainGameMode.mainGameMode_C|GetProgressionSystem _asmain_game_mode) "NewEnumerator7"))
      (:CastFailed
        _)))
  (return))

(fn SetInitialPosition
  (bind _foundedactor (CallFunction|GetActorwithIndex (Variables|Default|GetCurrentIndex)))
  (Transformation|SetActorTransform (Variables|Default|GetActiveCamera) (Transformation|GetActorTransform _foundedactor))
  (return))

(fn InitializeVariables
  (Variables|Default|SetCurrentIndex 0)
  (Variables|Default|SetNextIndex (+ (Variables|Default|GetCurrentIndex) 1))
  (bind _asmain_game_mode (Utilities|Casting|CastTomainGameMode (Game|GetGameMode))
    (:then
      (Variables|Default|SetActiveCamera (Variables|/Game/FirstPerson/Blueprints/mainGameMode.mainGameMode_C|GetActiveCamera _asmain_game_mode)))
    (:CastFailed
      _))
  (return))

(fn UpdateMovementPosition
  (Transformation|SetActorTransform (Variables|Default|GetActiveCamera) (Math|Transform|MakeTransform (+ (* (Variables|Default|GetMovementDirection) (Variables|Default|GetSpeed)) (Transformation|GetActorLocation (Variables|Default|GetActiveCamera))) (.DeviceRotation (Class|HeadMountedDisplayFunctionLibrary|GetOrientationandPosition)) "0, 0, 0"))
  (return))

(fn CheckImediatteMovementCondition
  (bind _foundedactor (CallFunction|GetActorwithIndex (Variables|Default|GetNextIndex)))
  (if (Variables|/Game/Blueprints/Logic/MovementSystem/BP_MovementTargetPoint.BP_MovementTargetPoint_C|GetImmediateMovement _foundedactor)
    (CallFunction|UpdateBorderPoints)
    (CallFunction|AddFactsfromCurrentPoint)
    (Transformation|SetActorTransform (Variables|Default|GetActiveCamera) (Math|Transform|MakeTransform (Variables|Default|GetNextPosition) (.DeviceRotation (Class|HeadMountedDisplayFunctionLibrary|GetOrientationandPosition)) "0, 0, 0"))
    (CallFunction|SetNewNextMovementPoint)
    (Variables|Default|SetSpeed (Variables|/Game/Blueprints/Logic/MovementSystem/BP_MovementTargetPoint.BP_MovementTargetPoint_C|GetSpeedInPoint _foundedactor)))
  (return))

(fn UpdateTransformationfromHeadDevice
  (bind _activecamera (Variables|Default|GetActiveCamera))
  (Transformation|SetActorTransform _activecamera (Math|Transform|MakeTransform (Transformation|GetActorLocation _activecamera) (.DeviceRotation (Class|HeadMountedDisplayFunctionLibrary|GetOrientationandPosition))))
  (return))

(fn ResetHeadDeviceTransform
  (Class|HeadMountedDisplayFunctionLibrary|ResetOrientationandPosition 0.0 "OrientationAndPosition")
  (return))

(fn SetInitialSpeed
  (bind _foundedactor (CallFunction|GetActorwithIndex (Variables|Default|GetCurrentIndex)))
  (bind _asbp_movement_target_point (Utilities|Casting|CastToBP_MovementTargetPoint _foundedactor))
  (Variables|Default|SetSpeed (Variables|/Game/Blueprints/Logic/MovementSystem/BP_MovementTargetPoint.BP_MovementTargetPoint_C|GetSpeedInPoint _asbp_movement_target_point)))

(fn UpdateMovementSpeed
  ;[1 1 1] Get start speed
  (bind _foundedactor (CallFunction|GetActorwithIndex (Variables|Default|GetCurrentIndex)))
  (bind _asbp_movement_target_point (Utilities|Casting|CastToBP_MovementTargetPoint _foundedactor))
  (LocalVariables|SetStartSpeed (Variables|/Game/Blueprints/Logic/MovementSystem/BP_MovementTargetPoint.BP_MovementTargetPoint_C|GetSpeedInPoint _asbp_movement_target_point))
  ;[1 1 1] Get target speed
  (bind _foundedactor_2 (CallFunction|GetActorwithIndex (Variables|Default|GetNextIndex)))
  (bind _asbp_movement_target_point_2 (Utilities|Casting|CastToBP_MovementTargetPoint _foundedactor_2))
  (LocalVariables|SetTargetSpeed (Variables|/Game/Blueprints/Logic/MovementSystem/BP_MovementTargetPoint.BP_MovementTargetPoint_C|GetSpeedInPoint _asbp_movement_target_point_2))
  (LocalVariables|SetDistanceBetweenPoints (Math|Vector|VectorLength (- (Variables|Default|GetNextPosition) (Variables|Default|GetCurrentPosition))))
  (LocalVariables|SetCameraDistanceToTargetPoint (Math|Vector|VectorLength (- (Variables|Default|GetNextPosition) (Transformation|GetActorLocation (Variables|Default|GetActiveCamera)))))
  (LocalVariables|SetDistanceRatio (- 1.0 (/ (LocalVariables|GetCameraDistanceToTargetPoint) (LocalVariables|GetDistanceBetweenPoints))))
  (bind _output_get (Variables|Default|SetSpeed (+ (LocalVariables|GetStartSpeed) (* (- (LocalVariables|GetTargetSpeed) (LocalVariables|GetStartSpeed)) (LocalVariables|GetDistanceRatio)))))
  (Development|PrintString (Utilities|String|ToString(Float) _output_get)))

(fn AddFactsfromCurrentPoint
  (bind _foundedactor (CallFunction|GetActorwithIndex (Variables|Default|GetCurrentIndex)))
  (bind _asmain_game_mode (Utilities|Casting|CastTomainGameMode (Game|GetGameMode)))
  (for _array_element (Variables|/Game/Blueprints/Logic/MovementSystem/BP_MovementTargetPoint.BP_MovementTargetPoint_C|GetFactsToAdd _foundedactor)
    (Default|AddFact (Variables|/Game/FirstPerson/Blueprints/mainGameMode.mainGameMode_C|GetProgressionSystem _asmain_game_mode) _array_element))
  (return))

(fn ChangeTargetPointtoNext
  (CallFunction|CheckStopMovementCondition)
  (CallFunction|SetNewNextMovementPoint)
  (CallFunction|CheckImediatteMovementCondition)
  (CallFunction|CheckLastPointCondition)
  (CallFunction|UpdateBorderPoints)
  (CallFunction|AddFactsfromCurrentPoint))

(fn CheckFactExists
  (params (FactName :type E_Facts%20Enum :default "NewEnumerator0"))
  (return false))